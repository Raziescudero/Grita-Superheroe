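; BP_Receptor is an actor that receives OSC messages and relays them as movement commands to the superhero character.
; On BeginPlay it finds BP_SuperHeroe and starts a local OSC server named "Voz" (voice), listening on localhost.
; Each received message's first string is passed to the hero's Movimiento function and printed on screen for debugging.
; The OSC address is not checked, so every message is treated as a command.
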(event Custom|AlRecibirMensaje
  (params (Message :type OSC%20Message%20Structure%20%28by%20ref%29) (IPAddress :type String) (Port :type Integer))
  (bind _value (Class|OSCManager|GetString Message))
  (Default|Movimiento (Variables|Default|GetHeroe) _value)
  (Development|PrintString _value))

(event EventBeginPlay
  (bind _returnvalue (Actor|GetActorOfClass "/Game/ThirdPerson/Blueprints/BP_SuperHeroe.BP_SuperHeroe_C"))
  (Variables|Default|SetHeroe _returnvalue)
  (bind _returnvalue_2 (Class|OSCManager|CreateOSCServer "127.0.0.1" 8000 false true "Voz" 0))
  (Variables|Default|SetServidorOSC _returnvalue_2)
  (EventDispatchers|AssignOnOscMessageReceived (Variables|Default|GetServidorOSC) (delegate Custom|AlRecibirMensaje)))

(event Collision|EventActorBeginOverlap
  (params (OtherActor :type Actor%20Object%20Reference)))

(event EventTick
  (params (DeltaSeconds :type Float%20%28single-precision%29)))

(fn ConstructionScript)